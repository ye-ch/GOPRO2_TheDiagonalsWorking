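; BP_DropZone is a capture-the-flag drop zone where Ghost players score by delivering the flag.
; When a BP_Ghost carrying the flag overlaps its Box, it clears HasFlag, increments GhostScore on CTF_GameMode and calls GhostScoring.
; A leftover CheckForWinG event, marked for deletion, holds win-screen and pause logic behind constant conditions that never pass.
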(event `self. Box.OnComponentBeginOverlap`
  (params (OverlappedComponent :type "PrimitiveComponent Object Reference") (OtherActor :type "Actor Object Reference") (OtherComp :type "PrimitiveComponent Object Reference") (OtherBodyIndex :type Integer) (bFromSweep :type Boolean) (SweepResult :type "HitResult Structure (by ref)"))
  (bind _asbp_ghost (cast `/Game/TopDown/Blueprints/BP_Ghost` OtherActor))
  (if (`/Game/TopDown/Blueprints/BP_Ghost.bHasFlag` _asbp_ghost)
    (set `/Game/TopDown/Blueprints/BP_Ghost.bHasFlag` false _asbp_ghost)
    (bind _asctf_game_mode (cast `/Game/CustomStuff/GameMode/CTF_GameMode` (`GameplayStatics.GetGameMode`)))
    (set `/Game/CustomStuff/GameMode/CTF_GameMode.GhostScore` (+ (`/Game/CustomStuff/GameMode/CTF_GameMode.GhostScore` _asctf_game_mode) 1) _asctf_game_mode)
    (`/Game/CustomStuff/GameMode/CTF_GameMode.GhostScoring` _asctf_game_mode)))

(event `CheckForWinG`
  ;[1 0 0] DELETE AFTER FIX
  (if (>= 0 2)
    (`WidgetLayoutLibrary.RemoveAllWidgets`)
    (bind _returnvalue (`|CreateWidget` "/Game/TopDown/Blueprints/WBP_GhostWin.WBP_GhostWin_C"))
    (`UserWidget.AddToViewport` _returnvalue 0)
    (`GameplayStatics.SetGamePaused` true :!label _label)
    (elif (>= 0 2)
      (`WidgetLayoutLibrary.RemoveAllWidgets`)
      (bind _returnvalue_2 (`|CreateWidget` "/Game/TopDown/Blueprints/WBP_HunterWin.WBP_HunterWin_C"))
      (`UserWidget.AddToViewport` _returnvalue_2 0)
      (goto _label))))

(fn `UserConstructionScript`)