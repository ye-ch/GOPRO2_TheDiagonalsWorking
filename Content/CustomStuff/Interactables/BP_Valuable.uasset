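; BP_Valuable is a capture-the-flag pickup that a BP_Ghost collects by overlapping its capsule.
; If the ghost has no flag, it sets HasFlag and destroys itself, subject to a team check.
; That check reads player states at hardcoded indices 1, then 3, rather than the overlapping ghost's, and requires the first team enum value.
; BeginPlay caches the CTF game mode, which is otherwise unused here.
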(event `self.ReceiveBeginPlay`
  (bind _asctf_game_mode (cast `/Game/CustomStuff/GameMode/CTF_GameMode` (`GameplayStatics.GetGameMode`)))
  (set `self.GameModeRef` _asctf_game_mode))

(event `self.Capsule.OnComponentBeginOverlap`
  (params (OverlappedComponent :type "PrimitiveComponent Object Reference") (OtherActor :type "Actor Object Reference") (OtherComp :type "PrimitiveComponent Object Reference") (OtherBodyIndex :type Integer) (bFromSweep :type Boolean) (SweepResult :type "HitResult Structure (by ref)"))
  (bind _asbp_ghost (cast `/Game/TopDown/Blueprints/BP_Ghost` OtherActor))
  (bind _asbp_player_state (cast `/Game/CustomStuff/GameMode/BP_PlayerState` (`GameplayStatics.GetPlayerState` 1))
    (:`then`
      (if (`|EnumEquality` (`/Game/CustomStuff/GameMode/BP_PlayerState.Team` _asbp_player_state) "NewEnumerator0")
        (if (not (`/Game/TopDown/Blueprints/BP_Ghost.bHasFlag` _asbp_ghost))
          ;[1 1 1] Make valuable visible on gost
          (set `/Game/TopDown/Blueprints/BP_Ghost.bHasFlag` true _asbp_ghost)
          (`self.K2_DestroyActor`))
        (else
          (bind _asbp_player_state_2 (cast `/Game/CustomStuff/GameMode/BP_PlayerState` (`GameplayStatics.GetPlayerState` 3)))
          (if (`|EnumEquality` (`/Game/CustomStuff/GameMode/BP_PlayerState.Team` _asbp_player_state_2) "NewEnumerator0")
            (if (not (`/Game/TopDown/Blueprints/BP_Ghost.bHasFlag` _asbp_ghost))
              ;[1 1 1] Make valuable visible on gost
              (set `/Game/TopDown/Blueprints/BP_Ghost.bHasFlag` true _asbp_ghost)
              (`self.K2_DestroyActor`))
            (else
              (`KismetSystemLibrary.PrintString` "wrong team"))))))
    (:`CastFailed`
      (`KismetSystemLibrary.PrintString` "playerstate cast failed"))))

(fn `UserConstructionScript`)